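; PlayerOneButton is a clickable button actor for a minigame that awards points to player one.
; On BeginPlay it casts and caches the ButtonsPC player controller and the GameplayGM game mode.
; Each click on its Cube component increments PlayerOneScore on the controller, unless that controller's TimesUp flag is set.
; The cached game mode reference is not used in the scoring logic.
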(event OnClicked(Cube)
  (params (TouchedComponent :type Primitive%20Component%20Object%20Reference) (ButtonPressed :type Key%20Structure))
  (bind _playercontrollerref (Variables|Default|GetPlayerControllerRef))
  (if (not (Variables|/Game/Blueprints/PlayerControllers/ButtonsPC.ButtonsPC_C|GetTimesUp (Variables|Default|GetPlayerControllerRef)))
    (bind _result (Math|Integer|IncrementInt (Variables|/Game/Blueprints/PlayerControllers/ButtonsPC.ButtonsPC_C|GetPlayerOneScore _playercontrollerref))
      (:%20%20
        (Variables|/Game/Blueprints/PlayerControllers/ButtonsPC.ButtonsPC_C|SetPlayerOneScore _playercontrollerref _result)))))

(event EventBeginPlay
  (bind _asbuttons_pc (Utilities|Casting|CastToButtonsPC (Game|GetPlayerController 0)))
  (Variables|Default|SetPlayerControllerRef _asbuttons_pc)
  (bind _asgameplay_gm (Utilities|Casting|CastToGameplayGM (Game|GetGameMode)))
  (Variables|Default|SetGameModeRef _asgameplay_gm))

(event Collision|EventActorBeginOverlap
  (params (OtherActor :type Actor%20Object%20Reference)))

(event EventTick
  (params (DeltaSeconds :type Float%20%28single-precision%29)))

(fn ConstructionScript)