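; HotBall is a clickable ball actor for a two-player minigame, passed back and forth between the players' sides.
; SetUpBallLocalization picks the starting side from PlayerOneStarts, then teleports the ball to a random spawn transform on that side.
; Each sphere click moves it to a random point on the opposite side and updates WhichSide, until the GameplayPC's TimesUp flag is set.
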(event OnClicked(Sphere)
  (params (TouchedComponent :type Primitive%20Component%20Object%20Reference) (ButtonPressed :type Key%20Structure))
  (if (not (Variables|/Game/Blueprints/GameplayPC.GameplayPC_C|GetTimesUp (Variables|Default|GetPlayerControllerRef)))
    (if (Utilities|Enum|Equal(Enum) (Variables|Default|GetWhichSide) "PlayerOne")
      (CallFunction|SetBallonPlayerTwoSide)
      (Variables|Default|SetWhichSide "PlayerTwo")
      (else
        (CallFunction|SetBallonPlayerOneSide)
        (Variables|Default|SetWhichSide "PlayerOne")))))

(event Custom|SetBallOnPlayerTwoSide
  (bind _playertwospawnpoints (Variables|Default|GetPlayerTwoSpawnPoints))
  (Transformation|SetActorTransform (Utilities|Array|Get(acopy) _playertwospawnpoints (Math|Random|RandomIntegerinRange 0 (- (Utilities|Array|Length _playertwospawnpoints) 1)))))

(event Custom|SetBallOnPlayerOneSide
  (bind _playeronespawnpoints (Variables|Default|GetPlayerOneSpawnPoints))
  (Transformation|SetActorTransform (Utilities|Array|Get(acopy) _playeronespawnpoints (Math|Random|RandomIntegerinRange 0 (- (Utilities|Array|Length _playeronespawnpoints) 1)))))

(event Custom|SetUpBallLocalization
  (if (Variables|Default|GetPlayerOneStarts?)
    (CallFunction|SetBallonPlayerOneSide)
    (Variables|Default|SetWhichSide "PlayerOne")
    (else
      (CallFunction|SetBallonPlayerTwoSide)
      (Variables|Default|SetWhichSide "PlayerTwo"))))

(event EventBeginPlay
  (bind _asgameplay_pc (Utilities|Casting|CastToGameplayPC (Game|GetPlayerController 0)))
  (Variables|Default|SetPlayerControllerRef _asgameplay_pc))

(fn ConstructionScript)