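; ButtonsPC is a player controller that runs a timed two-player minigame round and decides its winner.
; A looping one-second timer counts down SecondsLeft; at zero it compares both player scores, sets the result text and shows the winner bar.
; The winner's tally in GameInfoInstance is incremented, and after a short delay the MiniGamesConnector level opens.
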(event Custom|DecreseSeconds
  (bind _result (Math|Integer|DecrementInt (Variables|Default|GetSeconds%20Left))
    (:%20%20
      (bind _output_get (Variables|Default|SetSeconds%20Left _result))
      (if (== _output_get 0)
        (Variables|Default|SetTimesUp true)
        (CallFunction|CompareScore)
        (Variables|Default|SetWinnerBarVis "Visible")
        (Utilities|FlowControl|Delay 2.0)
        (Game|OpenLevel(byName) "MiniGamesConnector")))))

(event Custom|CompareScore
  (bind _gameinstanceref (Variables|Default|GetGameInstanceRef))
  (Math|Integer|CompareInt (Variables|Scores|GetPlayerOneScore) (Variables|Scores|GetPlayerTwoScore)
    (:>
      (Variables|Default|SetResult "The Winner Is: Player One!")
      (Math|Integer|IncrementInt (Variables|/Game/Blueprints/GameInfoInstance.GameInfoInstance_C|GetPlayerOneScore _gameinstanceref)))
    (:==
      (Variables|Default|SetResult "Draw!"))
    (:<
      (Variables|Default|SetResult "The Winner Is: Player Two!")
      (Math|Integer|IncrementInt (Variables|/Game/Blueprints/GameInfoInstance.GameInfoInstance_C|GetPlayerTwoScore _gameinstanceref)))))

(event EventBeginPlay
  (bind _asgame_info_instance (Utilities|Casting|CastToGameInfoInstance (Game|GetGameInstance)))
  (Variables|Default|SetGameInstanceRef _asgame_info_instance)
  (Utilities|Time|SetTimerbyFunctionName 0 "DecreseSeconds" 1.0 (not (Variables|Default|GetTimesUp))))

(fn ConstructionScript)